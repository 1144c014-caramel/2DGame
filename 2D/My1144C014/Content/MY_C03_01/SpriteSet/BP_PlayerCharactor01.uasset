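; Player character for a 2D side-scrolling game, with Enhanced Input movement and jumping, a base UI created on BeginPlay, and NPC interaction.
; Movement runs along world X while ConMove is true, flipping the sprite by rotation to face the input direction.
; Interact looks up BP_NPC_03 and shows its dialogue widget if the player is in range.
; Any damage subtracts from HP, with no death handling here.
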(event Custom|SetUI_NPC03
  (bind _returnvalue (UserInterface|CreateWidget "/Game/MY_C03_01/NPC/Widget/UI_ForNPC03.UI_ForNPC03_C"))
  (Widget|SetVisibility (Variables|/Game/MY_C03_01/NPC/Widget/UI_ForNPC03.UI_ForNPC03_C|GetTxt_NPCTalk _returnvalue) "Visible")
  (UserInterface|Viewport|AddtoViewport _returnvalue 0))

(event Custom|set%20uiNPCGuideRemove
  (Widget|RemovefromParent (stale Custom|SetUI_NPC03 _returnvalue)))

(event Custom|SetUIBase
  (bind _returnvalue (UserInterface|CreateWidget "/Game/MY_C03_01/SpriteSet/UI_Base.UI_Base_C"))
  (UserInterface|Viewport|AddtoViewport _returnvalue 0))

(event Input|EnhancedActionEvents|EnhancedInputActionIA_Move01
  (params (ActionValue :type Vector%202D%20Structure) (ElapsedSeconds :type Float%20%28double-precision%29) (TriggeredSeconds :type Float%20%28double-precision%29) (InputAction :type Input%20Action%20Object%20Reference :default "/Game/MY_C03_01/SpriteSet/Input/IA_Move01.IA_Move01"))
  (bind _x (Math|Vector2D|BreakVector2D ActionValue))
  (bind _playersprite (Variables|Default|GetPlayerSprite))
  (if (Variables|Default|GetConMove)
    (if (> _x 0.0)
      (Variables|Default|SetisFacingRight true)
      (else
        (Variables|Default|SetisFacingRight false)))
    (Pawn|Input|AddMovementInput "1.000000,0.000000,0.000000" _x false)
    (if (Variables|Default|GetisFacingRight)
      (Transformation|SetRelativeRotation _playersprite "0, 0, 0" false false)
      (else
        (Transformation|SetRelativeRotation _playersprite "0.000000,180.000000,0.000000" false false)))
    (else
      (Development|PrintString "Move Locked"))))

(event Input|EnhancedActionEvents|EnhancedInputActionIA_Interact
  (params (ActionValue :type Boolean) (ElapsedSeconds :type Float%20%28double-precision%29) (TriggeredSeconds :type Float%20%28double-precision%29) (InputAction :type Input%20Action%20Object%20Reference :default "/Game/MY_C03_01/SpriteSet/Input/IA_Interact.IA_Interact"))
  (:Started
    (bind _returnvalue (Actor|GetActorOfClass "/Game/MY_C03_01/NPC/BP_NPC_03.BP_NPC_03_C"))
    (bind _asbp_npc_03 (Utilities|Casting|CastToBP_NPC_03 _returnvalue))
    (if (Variables|/Game/MY_C03_01/NPC/BP_NPC_03.BP_NPC_03_C|GetPlayerInRange _asbp_npc_03)
      (CallFunction|SetUINPC03)
      (else
        (Development|PrintString "NoNPC")))))

(event Input|EnhancedActionEvents|EnhancedInputActionIA_Jump01
  (params (ActionValue :type Boolean) (ElapsedSeconds :type Float%20%28double-precision%29) (TriggeredSeconds :type Float%20%28double-precision%29) (InputAction :type Input%20Action%20Object%20Reference :default "/Game/MY_C03_01/SpriteSet/Input/IA_Jump01.IA_Jump01"))
  (:Started
    (Character|Jump))
  (:Completed
    (Character|StopJumping)))

(event EventBeginPlay
  (Input|AddMappingContext (PlayerController|LocalPlayerSubsystems|GetEnhancedInputLocalPlayerSubsystem (Game|GetPlayerController 0)) "/Game/MY_C03_01/SpriteSet/Input/IMC_Player01.IMC_Player01" 0 "(bIgnoreAllPressedKeysUntilRelease=True,bForceImmediately=False,bNotifyUserSettings=False)")
  (CallFunction|SetUIBase))

(event Collision|EventActorBeginOverlap
  (params (OtherActor :type Actor%20Object%20Reference)))

(event EventTick
  (params (DeltaSeconds :type Float%20%28single-precision%29)))

(event Game|Damage|EventAnyDamage
  (params (Damage :type Float%20%28single-precision%29) (DamageType :type Damage%20Type%20Object%20Reference) (InstigatedBy :type Controller%20Object%20Reference) (DamageCauser :type Actor%20Object%20Reference))
  (Variables|Default|SetHP (- (Variables|Default|GetHP) Damage)))

(fn ConstructionScript)