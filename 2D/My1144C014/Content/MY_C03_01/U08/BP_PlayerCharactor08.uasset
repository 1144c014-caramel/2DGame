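; Player character for a Paper2D side-scroller, with Enhanced Input movement along X, jumping, NPC interaction and level restart.
; Each tick it derives idle, walk or jump from movement to choose the flipbook, and input direction flips the sprite's X scale.
; It creates the base UI and NPC dialogue widget.
; Zero HP reloads Level03_02, while separate functions handle checkpoints, teleport respawn and level finish.
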(event Custom|SetUI_NPC03
  (bind _returnvalue (UserInterface|CreateWidget "/Game/MY_C03_01/NPC/Widget/UI_ForNPC03.UI_ForNPC03_C"))
  (Widget|SetVisibility (Variables|/Game/MY_C03_01/NPC/Widget/UI_ForNPC03.UI_ForNPC03_C|GetTxt_NPCTalk _returnvalue) "Visible")
  (UserInterface|Viewport|AddtoViewport _returnvalue 0))

(event Custom|set%20uiNPCGuideRemove
  (Widget|RemovefromParent (stale Custom|SetUI_NPC03 _returnvalue)))

(event Custom|SetUIBase
  (bind _returnvalue (UserInterface|CreateWidget "/Game/MY_C03_01/SpriteSet/UI_Base.UI_Base_C"))
  (UserInterface|Viewport|AddtoViewport _returnvalue 0))

(event Custom|SetStartLoc
  ;[0.15 0.15 0.15 0.5] Comment
  (Variables|Default|SetRespawnLocation (Transformation|GetActorLocation)))

(event Input|EnhancedActionEvents|EnhancedInputActionIA_Move01
  (params (ActionValue :type Vector%202D%20Structure) (ElapsedSeconds :type Float%20%28double-precision%29) (TriggeredSeconds :type Float%20%28double-precision%29) (InputAction :type Input%20Action%20Object%20Reference :default "/Game/MY_C03_01/SpriteSet/Input/IA_Move01.IA_Move01"))
  (bind _x (Math|Vector2D|BreakVector2D ActionValue))
  (Pawn|Input|AddMovementInput "1.000000,0.000000,0.000000" _x false)
  (CallFunction|UpdateFacingfromInput (* _x 0.3)))

(event Input|EnhancedActionEvents|EnhancedInputActionIA_Interact
  (params (ActionValue :type Boolean) (ElapsedSeconds :type Float%20%28double-precision%29) (TriggeredSeconds :type Float%20%28double-precision%29) (InputAction :type Input%20Action%20Object%20Reference :default "/Game/MY_C03_01/SpriteSet/Input/IA_Interact.IA_Interact"))
  (:Started
    (bind _returnvalue (Actor|GetActorOfClass "/Game/MY_C03_01/NPC/BP_NPC_03.BP_NPC_03_C"))
    (bind _asbp_npc_03 (Utilities|Casting|CastToBP_NPC_03 _returnvalue))
    (if (Variables|/Game/MY_C03_01/NPC/BP_NPC_03.BP_NPC_03_C|GetPlayerInRange _asbp_npc_03)
      (CallFunction|SetUINPC03)
      (else
        (Development|PrintString "NoNPC")))))

(event Input|EnhancedActionEvents|EnhancedInputActionIA_Jump01
  (params (ActionValue :type Boolean) (ElapsedSeconds :type Float%20%28double-precision%29) (TriggeredSeconds :type Float%20%28double-precision%29) (InputAction :type Input%20Action%20Object%20Reference :default "/Game/MY_C03_01/SpriteSet/Input/IA_Jump01.IA_Jump01"))
  (:Triggered
    (Character|Jump))
  (:Canceled
    (Character|StopJumping :!label _label))
  (:Completed
    (goto _label)))

(event Input|EnhancedActionEvents|EnhancedInputActionIA_Restart01
  (params (ActionValue :type Boolean) (ElapsedSeconds :type Float%20%28double-precision%29) (TriggeredSeconds :type Float%20%28double-precision%29) (InputAction :type Input%20Action%20Object%20Reference :default "/Game/MY_C03_01/SpriteSet/Input/IA_Restart01.IA_Restart01"))
  (Game|OpenLevel(byName) "Level03_02"))

(event EventBeginPlay
  (Utilities|FlowControl|Sequence
    (:then_0
      (Input|AddMappingContext (PlayerController|LocalPlayerSubsystems|GetEnhancedInputLocalPlayerSubsystem (Game|GetPlayerController 0)) "/Game/MY_C03_01/SpriteSet/Input/IMC_Player01.IMC_Player01" 0 "(bIgnoreAllPressedKeysUntilRelease=True,bForceImmediately=False,bNotifyUserSettings=False)")
      (CallFunction|SetUIBase)
      ;[0.15 0.15 0.15 0.5] Comment
      (CallFunction|UpdateMoveState)
      (CallFunction|PlayAnimation))
    (:then_1
      (CallFunction|ApplyFacing))
    (:then_2
      (CallFunction|SetStartLoc))))

(event Collision|EventActorBeginOverlap
  (params (OtherActor :type Actor%20Object%20Reference)))

(event Game|Damage|EventAnyDamage
  (params (Damage :type Float%20%28single-precision%29) (DamageType :type Damage%20Type%20Object%20Reference) (InstigatedBy :type Controller%20Object%20Reference) (DamageCauser :type Actor%20Object%20Reference))
  (Variables|Default|SetHP (- (Variables|Default|GetHP) Damage))
  (if (<= (Variables|Default|GetHP) 0.0)
    (Game|OpenLevel(byName) "Level03_02")))

(event EventTick
  (params (DeltaSeconds :type Float%20%28single-precision%29))
  (CallFunction|UpdateMoveState)
  (CallFunction|PlayAnimation))

(fn ConstructionScript)

(fn UpdateMoveState
  (if (AI|Components|NavMovement|IsFalling (Variables|Character|GetCharacterMovement))
    (Variables|Default|SetAninState "NewEnumerator2")
    (elif (> (Math|Float|Absolute(Float) (.X (Math|Vector|BreakVector (Transformation|GetVelocity)))) 5.0)
      (Variables|Default|SetAninState "NewEnumerator1")
      (else
        (Variables|Default|SetAninState "NewEnumerator0")))))

(fn PlayAnimation
  (bind _paperflipbook (Variables|Default|GetPaperFlipbook))
  (bind _paperflipbook_2 (Variables|Default|GetPaperFlipbook))
  (switch Utilities|FlowControl|Switch|SwitchonEnum_ChangeAnin (Variables|Default|GetAninState)
    (:NewEnumerator0
      (Sprite|SetFlipbook _paperflipbook_2 "/Game/MY_C03_01/U06/Flipbook/FB_Girl_Idle.FB_Girl_Idle"))
    (:NewEnumerator1
      (Sprite|SetFlipbook _paperflipbook_2 "/Game/MY_C03_01/U06/Flipbook/FB_Girll_Walk.FB_Girll_Walk"))
    (:NewEnumerator2
      (Sprite|SetFlipbook _paperflipbook_2 "/Game/MY_C03_01/U06/Flipbook/FB_Girl_Jump.FB_Girl_Jump")))
  (Components|Timeline|SetLooping _paperflipbook (Utilities|Enum|NotEqual(Enum) (Variables|Default|GetAninState) "NewEnumerator2"))
  (Audio|Components|Audio|Play _paperflipbook))

(fn ApplyFacing
  (Transformation|SetRelativeScale3D (Variables|Default|GetPaperFlipbook) (Math|Vector|MakeVector (Variables|Default|GetFacingSing) 0.3 0.3)))

(fn UpdateFacingfromInput
  (params (AxusValue :type Float%20%28double-precision%29))
  (if (> (Math|Float|Absolute(Float) AxusValue) 0.1)
    (Variables|Default|SetFacingSing (Math|Float|SelectFloat AxusValue -0.3 (> AxusValue 0.0)))
    (CallFunction|ApplyFacing)))

(fn SetCheckPoint
  (params (NewLocation :type Vector))
  (Variables|Default|SetRespawnLocation NewLocation))

(fn Respawn
  (Character|StopJumping)
  (Components|Movement|StopMovementImmediately (Variables|Character|GetCharacterMovement))
  (Variables|Default|SetMoveInputX 0.0)
  (Transformation|SetActorLocation (Variables|Default|GetRespawnLocation) false true)
  (Pawn|Components|CharacterMovement|SetMovementMode (Variables|Character|GetCharacterMovement) "MOVE_Walking" 0)
  (Variables|Default|SetAninState "NewEnumerator0")
  (Variables|Default|SetFacingSing 1.0))

(fn FinishLevel
  (Pawn|Components|CharacterMovement|DisableMovement (Variables|Character|GetCharacterMovement))
  (Variables|Default|SetAninState "NewEnumerator0")
  (Development|PrintString "Win  按下R重新開始遊戲"))